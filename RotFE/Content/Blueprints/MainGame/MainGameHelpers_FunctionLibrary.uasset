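; Blueprint function library of global getters for the main game's core objects.
; It returns the game state cast to MainGame_bpgs, player controller 0 cast to MainGame_bppc, and the WorldMapData held by that game state.
; Each getter uses a sequence whose first branch returns on success, so a failed cast or validity check falls through to print a long-lasting on-screen error and return empty.
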(fn GetMainGameState
  (Utilities|FlowControl|Sequence
    (:then_0
      ;[0 1 0.25] Success
      (bind _asmain_game_bpgs (Utilities|Casting|CastToMainGame_bpgs (Game|GetGameState)))
      (return _asmain_game_bpgs))
    (:then_1
      ;[1 0.1 0.1] Failure
      (Development|PrintString 0 "Main Game State does not exist!" true true "(R=0.000000,G=0.660000,B=1.000000,A=1.000000)" 99.0)
      (return 0))))

(fn GetMainGameController
  (Utilities|FlowControl|Sequence
    (:then_0
      ;[0 1 0.25] Success
      (bind _asmain_game_bppc (Utilities|Casting|CastToMainGame_bppc (Game|GetPlayerController 0)))
      (return _asmain_game_bppc))
    (:then_1
      ;[1 0.1 0.1] Failure
      (Development|PrintString 0 "Main Game Controller does not exist!" true true "(R=0.000000,G=0.660000,B=1.000000,A=1.000000)" 99.0)
      (return 0))))

(fn GetWorldMapData
  (bind _outgamestate (CallFunction|GetMainGameState))
  (bind _worldmapdata (Variables|/Game/Blueprints/MainGame/MainGame_bpgs.MainGame_bpgs_C|GetWorldMapData _outgamestate))
  (Utilities|FlowControl|Sequence
    (:then_0
      (Utilities|IsValid _worldmapdata
        (:Is%20Valid
          (return _worldmapdata))))
    (:then_1
      (Development|PrintString 0 "World Map Data does not exist!" true true "(R=0.000000,G=0.660000,B=1.000000,A=1.000000)" 99.0)
      (return 0))))