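; Player controller for the main game that creates the root UI and handles pause and escape input.
; On BeginPlay it runs the parent logic, then creates MainGameUIRoot_bpw, stores it and adds it to the viewport.
; Escape presses are forwarded to that root widget, while P toggles the game's paused state directly.
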(event EventBeginPlay
  (|CallParentFunction)
  (bind _returnvalue (UserInterface|CreateWidget "/Game/Blueprints/MainGame/UI/MainGameUIRoot_bpw.MainGameUIRoot_bpw_C"))
  (bind _output_get (Variables|Default|SetMainGameRootUI _returnvalue))
  (UserInterface|Viewport|AddtoViewport _output_get 0))

(event Input|KeyboardEvents|P
  (params (Key :type Key%20Structure :default "None"))
  (:Pressed
    (CallFunction|ToggleGamePaused)))

(event Input|KeyboardEvents|Escape
  (params (Key :type Key%20Structure :default "None"))
  (:Pressed
    (Default|HandleEscapePressed (Variables|Default|GetMainGameRootUI) Key)))

(fn ConstructionScript)

(fn ToggleGamePaused
  (Game|SetGamePaused (not (Game|IsGamePaused))))