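; MainGame game state Blueprint that tracks total game time elapsed and the player's faction.
; On BeginPlay it copies both values from the current save, provided the game instance and save are valid.
; Tick then adds delta seconds to the elapsed time each frame; nothing here writes the values back to the save.
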(event EventBeginPlay
  (bind _outsave (CallFunction|GetCurrentSave))
  (Utilities|IsValid (Game|GetGameInstance)
    (:Is%20Valid
      (Utilities|IsValid _outsave
        (:Is%20Valid
          (Variables|Default|SetGameTimeElapsed (Variables|/Game/Blueprints/RotFE_Save.RotFE_Save_C|GetGameTimeElapsed _outsave))
          (Variables|Default|SetPlayerFaction (Variables|/Game/Blueprints/RotFE_Save.RotFE_Save_C|GetPlayerFaction _outsave)))))))

(event EventTick
  (params (DeltaSeconds :type Float%20%28single-precision%29))
  (Variables|Default|SetGameTimeElapsed (+ DeltaSeconds (Variables|Default|GetGameTimeElapsed))))

(fn ConstructionScript)