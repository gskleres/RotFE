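; String function library whose FormatSeconds function turns a number of seconds into a clock-style time string.
; It derives hours, minutes and seconds with division, modulo and truncation, then joins them with colons through Append and SelectString.
; The hour segment appears only when nonzero, minutes are zero-padded only when hours show, and seconds below ten always get a leading zero.
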(fn FormatSeconds
  (params (InSeconds :type Float%20%28single-precision%29))
  (bind _returnvalue (/ InSeconds 3.6e+03))
  (bind _returnvalue_2 (Math|Float|%(Float) InSeconds 3.6e+03))
  (bind _returnvalue_3 (Math|Float|Truncate _returnvalue))
  (bind _returnvalue_4 (/ _returnvalue_2 6e+01))
  (bind _returnvalue_5 (Math|Float|%(Float) _returnvalue_2 6e+01))
  (bind _returnvalue_6 (Math|Float|Truncate _returnvalue_4))
  (bind _returnvalue_7 (Math|Float|Truncate _returnvalue_5))
  (bind _returnvalue_8 (> _returnvalue_3 0))
  (return (Utilities|String|Append (Utilities|String|SelectString (Utilities|String|Append (Utilities|String|ToString(Integer) _returnvalue_3) ":") "" _returnvalue_8) (Utilities|String|Append (Utilities|String|SelectString "0" "" (and _returnvalue_8 (< _returnvalue_6 10))) (Utilities|String|ToString(Integer) _returnvalue_6) ":") (Utilities|String|Append (Utilities|String|SelectString "0" "" (< _returnvalue_7 10)) (Utilities|String|ToString(Integer) _returnvalue_7)))))