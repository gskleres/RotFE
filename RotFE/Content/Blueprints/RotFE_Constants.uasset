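; RotFE_Constants is a set of shared helper functions for RotFE that exposes a constant and common framework accessors.
; It returns the default save game name prefix and fetches the game state and game instance, cast to MainGame_bpgs and RotFE_GameInstance.
; Each getter uses a Sequence to return the cast result, falling through on failure to a Print String error and an empty return.
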(fn GetRotFESaveGamePrefix
  (return "RotFE_default"))

(fn GetMainGameState
  (Utilities|FlowControl|Sequence
    (:then_0
      ;[0 1 0.25] Success
      (bind _asmain_game_bpgs (Utilities|Casting|CastToMainGame_bpgs (Game|GetGameState)))
      (return _asmain_game_bpgs))
    (:then_1
      ;[1 0.1 0.1] Failure
      (Development|PrintString 0 "Main Game State does not exist!" true true "(R=0.000000,G=0.660000,B=1.000000,A=1.000000)" 99.0)
      (return 0))))

(fn GetRotFEGameInstance
  (Utilities|FlowControl|Sequence
    (:then_0
      ;[0 1 0.25] Success
      (bind _asrot_fe_game_instance (Utilities|Casting|CastToRotFE_GameInstance (Game|GetGameInstance)))
      (return _asrot_fe_game_instance))
    (:then_1
      ;[1 0.1 0.1] Failure
      (Development|PrintString 0 "Cast of game instance failed!" false true "(R=0.000000,G=0.660000,B=1.000000,A=1.000000)" 99.0)
      (return 0))))