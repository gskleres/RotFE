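; DataHelpers is a set of helper functions supplying the save game name prefix and lists of the game's valid factions.
; GetAllValidFactionDataRows reads FactionsDataTable and skips the first row by index, assuming it is NO_FACTION, then returns the unique remaining rows.
; The enum and display name getters build on that list, extracting each row's FactionType or DisplayName into unique arrays.
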(fn GetSaveGamePrefix
  (return "RotFE"))

(fn GetAllValidFactionDataRows
  (Utilities|FlowControl|Sequence
    (:then_0
      ;[0.5 0.5 0.5] Get every faction data row except NO_FACTION
      (bind _outrownames (DataTable|GetDataTableRowNames "/Game/Blueprints/GameData/FactionsDataTable.FactionsDataTable"))
      (for (_array_element _array_index) _outrownames
        (if (> _array_index 0)
          (bind _returnvalue (Utilities|GetDataTableRow "/Game/Blueprints/GameData/FactionsDataTable.FactionsDataTable" _array_element)
            (:then
              (Utilities|Array|AddUnique (LocalVariables|GetL_FactionList) _returnvalue))))))
    (:then_1
      (return (LocalVariables|GetL_FactionList)))))

(fn GetAllValidFactionEnums
  (Utilities|FlowControl|Sequence
    (:then_0
      ;[0.5 0.5 0.5] Collect all of the enums
      (for _array_element (FactionData|GetAllValidFactionDataRows)
        (Utilities|Array|AddUnique (LocalVariables|GetL_FactionList) (.FactionType (Utilities|Struct|BreakFactionData _array_element)))))
    (:then_1
      (return (LocalVariables|GetL_FactionList)))))

(fn GetAllValidFactionDisplayNames
  (Utilities|FlowControl|Sequence
    (:then_0
      ;[0.5 0.5 0.5] Collect all the faction DisplayNames
      (for _array_element (FactionData|GetAllValidFactionDataRows)
        (Utilities|Array|AddUnique (LocalVariables|GetL_FactionList) (.DisplayName (Utilities|Struct|BreakFactionData _array_element)))))
    (:then_1
      (return (LocalVariables|GetL_FactionList)))))