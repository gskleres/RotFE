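; Save function library that creates, fetches and loads RotFE_Save objects for the game.
; MakeCurrentSave builds a new save object from the main game state's elapsed time and player faction, without writing it to disk.
; GetCurrentSave reads the save cached on RotFE_GameInstance.
; LoadSaveGame loads the prefix-named slot and uses a Sequence as a fallback, logging when the cast fails.
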(fn MakeCurrentSave
  (bind _outgamestate (CallFunction|GetMainGameState))
  (bind _returnvalue (SaveGame|CreateSaveGameObject "/Game/Blueprints/RotFE_Save.RotFE_Save_C"))
  (Variables|/Game/Blueprints/RotFE_Save.RotFE_Save_C|SetGameTimeElapsed _returnvalue (Variables|/Game/Blueprints/MainGame/MainGame_bpgs.MainGame_bpgs_C|GetGameTimeElapsed _outgamestate))
  (Variables|/Game/Blueprints/RotFE_Save.RotFE_Save_C|SetPlayerFaction _returnvalue (Variables|/Game/Blueprints/MainGame/MainGame_bpgs.MainGame_bpgs_C|GetPlayerFaction _outgamestate))
  (return _returnvalue))

(fn GetCurrentSave
  (bind _asrot_fe_game_instance (Utilities|Casting|CastToRotFE_GameInstance (Game|GetGameInstance))
    (:then
      (return (Variables|/Game/Blueprints/RotFE_GameInstance.RotFE_GameInstance_C|GetCurrentSave _asrot_fe_game_instance)))
    (:CastFailed
      (Development|PrintString 0 "Save Function Library: Could not get game instance!" true true "(R=0.000000,G=0.660000,B=1.000000,A=1.000000)" 99.0))))

(fn LoadSaveGame
  (Utilities|FlowControl|Sequence
    (:then_0
      ;[0 1 0.25] Success
      (bind _returnvalue (SaveGame|LoadGamefromSlot (CallFunction|GetRotFESaveGamePrefix)))
      (bind _asrot_fe_save (Utilities|Casting|CastToRotFE_Save _returnvalue))
      (return _asrot_fe_save))
    (:then_1
      ;[1 0.1 0.1] Failure
      (Development|PrintString 0 "Cast of save game failed!" false true "(R=0.000000,G=0.660000,B=1.000000,A=1.000000)" 99.0)
      (return 0))))